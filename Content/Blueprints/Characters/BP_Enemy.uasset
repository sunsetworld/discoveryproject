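; BP_Enemy is an enemy character that chases the BP_Player found at BeginPlay.
; Every Tick it reissues AI MoveTo toward the player while that reference is valid and resets its rotation to zero.
; Two overlap components react to the player: KillCollision subtracts one Health from the player and destroys the enemy, while JumpCollision makes the enemy jump.
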(event `self.ReceiveBeginPlay`
  (bind _returnvalue (`GameplayStatics.GetActorOfClass` "/Game/Blueprints/Characters/BP_Player.BP_Player_C"))
  (set `self.BP_Player` _returnvalue))

(event `self.ReceiveTick`
  (params (DeltaSeconds :type "Float (single-precision)"))
  (bind _bp_player (`self.BP_Player`))
  (`/Engine/EditorBlueprintResources/StandardMacros.IsValid` _bp_player
    (:`Is Valid`
      (`|AIMoveTo` self (0.0 0.0 0.0) _bp_player
        (:`then`
          (`self.K2_SetActorRotation` (struct)))))))

(event `self.KillCollision.OnComponentBeginOverlap`
  (params (OverlappedComponent :type "PrimitiveComponent Object Reference") (OtherActor :type "Actor Object Reference") (OtherComp :type "PrimitiveComponent Object Reference") (OtherBodyIndex :type Integer) (bFromSweep :type Boolean) (SweepResult :type "HitResult Structure (by ref)"))
  (bind _asbp_player (cast `/Game/Blueprints/Characters/BP_Player` OtherActor))
  (`/Engine/EditorBlueprintResources/StandardMacros.DecrementInt` (`/Game/Blueprints/Characters/BP_Player.Health` _asbp_player)
    (:`  `
      (`self.K2_DestroyActor`))))

(event `self.JumpCollision.OnComponentBeginOverlap`
  (params (OverlappedComponent :type "PrimitiveComponent Object Reference") (OtherActor :type "Actor Object Reference") (OtherComp :type "PrimitiveComponent Object Reference") (OtherBodyIndex :type Integer) (bFromSweep :type Boolean) (SweepResult :type "HitResult Structure (by ref)"))
  (cast `/Game/Blueprints/Characters/BP_Player` OtherActor)
  (`self.Jump`))

(fn `UserConstructionScript`)