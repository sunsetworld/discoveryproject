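; BP_Jerry is an NPC that shows dialogue text while the player is near.
; On BeginPlay it hides NPCTxt, stores the dialogue array's length and sets the text to the current index's entry.
; Overlaps of PlayerNPCCollision with BP_Player toggle the text's visibility and the TextIsVisible flag.
; SetDialogueTxt displays an entry by index, but nothing in this graph advances the dialogue.
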(event `self.ReceiveBeginPlay`
  (`SceneComponent.SetVisibility` (`self.NPCTxt`) false false)
  (set `self.MaxDialogueTxtNumber` (`KismetArrayLibrary.Array_Length` (`self.DialogueTxt`)))
  (`self.SetDialogueTxt` (`self.DialogueTxtNumber`)))

(event `self.ReceiveTick`
  (params (DeltaSeconds :type "Float (single-precision)")))

(event `self.PlayerNPCCollision.OnComponentBeginOverlap`
  (params (OverlappedComponent :type "PrimitiveComponent Object Reference") (OtherActor :type "Actor Object Reference") (OtherComp :type "PrimitiveComponent Object Reference") (OtherBodyIndex :type Integer) (bFromSweep :type Boolean) (SweepResult :type "HitResult Structure (by ref)"))
  (cast `/Game/Blueprints/Characters/BP_Player` OtherActor)
  (`SceneComponent.SetVisibility` (`self.NPCTxt`) true false)
  (set `self.textIsVisible` true))

(event `self.PlayerNPCCollision.OnComponentEndOverlap`
  (params (OverlappedComponent :type "PrimitiveComponent Object Reference") (OtherActor :type "Actor Object Reference") (OtherComp :type "PrimitiveComponent Object Reference") (OtherBodyIndex :type Integer))
  (cast `/Game/Blueprints/Characters/BP_Player` OtherActor)
  (`SceneComponent.SetVisibility` (`self.NPCTxt`) false false)
  (set `self.textIsVisible` false))

(fn `SetDialogueTxt`
  (params (DialogueTxt :type Integer))
  (`TextRenderComponent.K2_SetText` (`self.NPCTxt`) (`|GetArrayItem` (`self.DialogueTxt`) DialogueTxt)))

(fn `UserConstructionScript`)